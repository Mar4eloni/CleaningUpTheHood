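; BP_TrashCan is a trash can actor that the player cleans until it is gone.
; Overlapping its Perimeter with a 2DGoonCharacter enables the actor's input and opens a gate; leaving disables input and closes it.
; While the gate is open, each Clean press subtracts that character's cleaning strength from the garbage amount.
; Tick checks the amount and destroys the actor once it reaches zero or below.
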(event `self.ReceiveTick`
  (params (DeltaSeconds :type "Float (single-precision)"))
  (if (<= (`self.GarbageAmmount`) 0)
    (`self.K2_DestroyActor` self)))

(event `InputAction|Clean`
  (params (Key :type "Key Structure"))
  (:`Pressed`
    (`/Engine/EditorBlueprintResources/StandardMacros.Gate` true :!label _label
      (:`Exit`
        (set `self.GarbageAmmount` (- (`self.GarbageAmmount`) (`/Game/GameCharacter/2DGoonCharacter.CleaningStreinght` (stale `self.Perimeter.OnComponentBeginOverlap` _as2dgoon_character))))))))

(event `self.Perimeter.OnComponentBeginOverlap`
  (params (OverlappedComponent :type "PrimitiveComponent Object Reference") (OtherActor :type "Actor Object Reference") (OtherComp :type "PrimitiveComponent Object Reference") (OtherBodyIndex :type Integer) (bFromSweep :type Boolean) (SweepResult :type "HitResult Structure (by ref)"))
  (bind _as2dgoon_character (cast `/Game/GameCharacter/2DGoonCharacter` OtherActor))
  (`self.EnableInput` (`GameplayStatics.GetPlayerController` 0))
  (goto _label :!via `Open`))

(event `self.Perimeter.OnComponentEndOverlap`
  (params (OverlappedComponent :type "PrimitiveComponent Object Reference") (OtherActor :type "Actor Object Reference") (OtherComp :type "PrimitiveComponent Object Reference") (OtherBodyIndex :type Integer))
  (cast `/Game/GameCharacter/2DGoonCharacter` OtherActor)
  (`self.DisableInput` (`GameplayStatics.GetPlayerController` 0))
  (goto _label :!via `Close`))

(fn `UserConstructionScript`)