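; BP_Dzoger is an interactable pickup that grants the Dzoger to the 2DGoonCharacter.
; Box overlap with that character shows a hint, enables player input on the actor and opens a Gate; leaving reverses all three.
; Pressing Interaction passes through the Gate and a DoOnce to set the character's BhasDzoger flag, then destroys the pickup.
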(event `InputAction|Interaction` :consume false
  (params (Key :type "Key Structure"))
  (:`Pressed`
    (`/Engine/EditorBlueprintResources/StandardMacros.Gate` true :!label _label
      (:`Exit`
        (`/Engine/EditorBlueprintResources/StandardMacros.DoOnce` false
          (:`Completed`
            (set `/Game/GameCharacter/2DGoonCharacter.bhasDzoger` true (stale `self.Box.OnComponentBeginOverlap` _as2dgoon_character))
            (`self.K2_DestroyActor` self)))))))

(event `self.Box.OnComponentBeginOverlap`
  (params (OverlappedComponent :type "PrimitiveComponent Object Reference") (OtherActor :type "Actor Object Reference") (OtherComp :type "PrimitiveComponent Object Reference") (OtherBodyIndex :type Integer) (bFromSweep :type Boolean) (SweepResult :type "HitResult Structure (by ref)"))
  (bind _as2dgoon_character (cast `/Game/GameCharacter/2DGoonCharacter` OtherActor))
  (`SceneComponent.SetVisibility` (`self.Hint`) true false)
  (`self.EnableInput` (`GameplayStatics.GetPlayerController` 0))
  (goto _label :!via `Open`))

(event `self.Box.OnComponentEndOverlap`
  (params (OverlappedComponent :type "PrimitiveComponent Object Reference") (OtherActor :type "Actor Object Reference") (OtherComp :type "PrimitiveComponent Object Reference") (OtherBodyIndex :type Integer))
  (cast `/Game/GameCharacter/2DGoonCharacter` OtherActor)
  (`SceneComponent.SetVisibility` (`self.Hint`) false false)
  (`self.DisableInput` (`GameplayStatics.GetPlayerController` 0))
  (goto _label :!via `Close`))

(fn `UserConstructionScript`)